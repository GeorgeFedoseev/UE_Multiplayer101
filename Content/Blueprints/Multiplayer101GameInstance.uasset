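; Game instance Blueprint that handles LAN multiplayer sessions, exposing events to host, search for and join games.
; Hosting creates a two-connection session and searching finds LAN sessions, both through async session nodes using the first player controller.
; Results are printed on screen and broadcast through host and server-list success or failure calls, with found sessions passed along.
; The join event is an empty stub.
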(event `HOSTGame`
  ;[1 1 1] Host Game
  (`CreateSessionCallbackProxy.CreateSession` (`GameplayStatics.GetPlayerController` 0) 2 true
    (:`OnSuccess`
      (`KismetSystemLibrary.PrintString` "Session craeted successfully!" true true (struct :`G` 1.0 :`B` 0.304821 :`A` 1.0))
      (`self.HostedGame`))
    (:`OnFailure`
      (`KismetSystemLibrary.PrintString` "Failed to start session!" true true (struct :`R` 0.855 :`B` 0.008874 :`A` 1.0))
      (`self.HostGameFailed`))))

(event `SEARCHGames`
  ;[1 1 1] Find Game
  (bind _results (`FindSessionsCallbackProxy.FindSessions` (`GameplayStatics.GetPlayerController` 0) 0 true)
    (:`OnSuccess`
      (`self.OnServerListUpdated` _results)
      (`KismetSystemLibrary.PrintString` (`KismetStringLibrary.Concat_StrStr` (`KismetStringLibrary.Concat_StrStr` "Found: " (`KismetStringLibrary.Conv_IntToString` (`KismetArrayLibrary.Array_Length` _results))) " games")))
    (:`OnFailure`
      (`self.OnServerSearchFailed`)
      (`KismetSystemLibrary.PrintString` "Server search failed!" true true (struct :`R` 0.855 :`B` 0.008874 :`A` 1.0)))))

(event `JOIN GAME`)